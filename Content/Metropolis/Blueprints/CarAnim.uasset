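; CarAnim is a Blueprint that animates a car mesh along a spline path.
; On BeginPlay it applies the CarMat material, sets the timeline play rate from CarSpeed and plays it from the start.
; Each timeline update maps AnimationAlpha to a distance along the spline, setting the mesh's world location and rotation while keeping its scale.
; StopAnim toggles pause by switching the play rate between zero and CarSpeed.
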(event Custom|StopAnim
  (bind _timeline_0 (Variables|Default|GetTimeline_0))
  (if (Variables|Default|GetIsPaused)
    (Variables|Default|SetIsPaused false)
    (Components|Timeline|SetPlayRate _timeline_0 (Variables|Default|GetCarSpeed))
    (else
      (Variables|Default|SetIsPaused true)
      (Components|Timeline|SetPlayRate _timeline_0 0.0))))

(event EventBeginPlay
  (bind _spline (Variables|Default|GetSpline))
  (bind _staticmesh (Variables|Default|GetStaticMesh))
  (Rendering|Material|SetMaterial _staticmesh 0 (.MaterialInterface (Utilities|Struct|BreakStaticMaterial (Variables|Default|GetCarMat))))
  (Components|Timeline|SetPlayRate (Variables|Default|GetTimeline_0) (Variables|Default|GetCarSpeed))
  (bind _animationalpha (Timeline|Timeline_0 PlayFromStart)
    (:Update
      (Transformation|SetWorldTransform _staticmesh (Math|Transform|MakeTransform (Spline|GetLocationatDistanceAlongSpline _spline (* (Spline|GetSplineLength _spline) _animationalpha) "World") (Spline|GetRotationatDistanceAlongSpline _spline (* (Spline|GetSplineLength _spline) _animationalpha) "World") (Transformation|GetWorldScale _staticmesh)) false false))))

(event Collision|EventActorBeginOverlap
  (params (OtherActor :type Actor%20Object%20Reference)))

(event EventTick
  (params (DeltaSeconds :type Float%20%28single-precision%29)))

(fn ConstructionScript)